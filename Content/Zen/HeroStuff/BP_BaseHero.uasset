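; Base hero Blueprint that determines which of the hero's stats is highest when play begins.
; UpdateActiveSkill finds the index of the largest value in the Stats float array and maps the first five indices to matching enum values.
; BeginPlay stores that result in HighestStat, apparently to represent the hero's active skill, and nothing in this Blueprint recalculates it afterwards.
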(event EventBeginPlay
  (bind _highest_stat (CallFunction|UpdateActiveSkill (.Stats (Utilities|Struct|BreakS_HeroInfo (Variables|Default|GetStats)))))
  (Variables|Default|SetHighest%20Stat _highest_stat))

(fn ConstructionScript)

(fn UpdateActiveSkill
  (params (Hero%20Stats :type Array%20of%20Floats%20%28double-precision%29))
  (switch int (.IndexOfMaxValue (Math|Float|MaxOfFloatArray Hero%20Stats))
    (:0
      (return "NewEnumerator0"))
    (:1
      (return "NewEnumerator1"))
    (:2
      (return "NewEnumerator2"))
    (:3
      (return "NewEnumerator3"))
    (:4
      (return "NewEnumerator4"))))