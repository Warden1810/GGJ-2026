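; BP_Player is the player Blueprint that handles pause and hero inventory input.
; On BeginPlay it adds the IMC_Player Enhanced Input mapping context to BP_PlayerController.
; Both inputs first check the day state through a Game Mode message.
; When it is true, the pause input alternates pausing and unpausing the day via a FlipFlop, and the inventory input messages the HUD to set inventory visibility.
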(event Input|EnhancedActionEvents|EnhancedInputActionIA_PauseMenu
  (params (ActionValue :type Boolean) (ElapsedSeconds :type Float%20%28double-precision%29) (TriggeredSeconds :type Float%20%28double-precision%29) (InputAction :type Input%20Action%20Object%20Reference :default "/Game/Mechanics/Controls/Input_Actions/IA_PauseMenu.IA_PauseMenu"))
  (bind _returnvalue (Game|GetGameMode))
  (:Started
    (bind _day_ongoing_ (Class|BPIGameMode|GetDayState(Message) (Game|GetGameMode)))
    (if _day_ongoing_
      (Utilities|FlowControl|FlipFlop
        (:A
          (Class|BPIGameMode|PauseDay(Message) _returnvalue))
        (:B
          (Class|BPIGameMode|UnPauseDay(Message) _returnvalue))))))

(event Input|EnhancedActionEvents|EnhancedInputActionIA_HeroInventory
  (params (ActionValue :type Boolean) (ElapsedSeconds :type Float%20%28double-precision%29) (TriggeredSeconds :type Float%20%28double-precision%29) (InputAction :type Input%20Action%20Object%20Reference :default "/Game/Mechanics/Controls/Input_Actions/IA_HeroInventory.IA_HeroInventory"))
  (:Started
    (bind _day_ongoing_ (Class|BPIGameMode|GetDayState(Message) (Game|GetGameMode)))
    (if _day_ongoing_
      (Class|BPIHUD|SetHeroInventoryVisibility(Message) (CallFunction|GetHUD)))))

(event EventBeginPlay
  (bind _asbp_player_controller (Utilities|Casting|CastToBP_PlayerController (Game|GetPlayerController 0)))
  (Input|AddMappingContext (PlayerController|LocalPlayerSubsystems|GetEnhancedInputLocalPlayerSubsystem _asbp_player_controller) "/Game/Mechanics/Controls/IMC_Player.IMC_Player" 0 "(bIgnoreAllPressedKeysUntilRelease=True,bForceImmediately=False,bNotifyUserSettings=False)"))

(fn ConstructionScript)