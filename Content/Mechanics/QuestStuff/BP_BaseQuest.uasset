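; Base quest Blueprint that runs one randomly picked quest from offer to success or failure.
; A picked quest starts an expiry timer, which accepting clears and which only prints a message on timeout.
; Starting chains timers for the quest's travel and duration, then tests a random point generated from its required stats to decide the outcome.
; Success and failure events are empty, and the heroes passed on start are unused.
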(event Custom|QuestTimeout
  (Development|PrintString "Quest Scaduta"))

(event Custom|AcceptQuest
  (Utilities|Time|ClearandInvalidateTimerbyHandle (Variables|Default|GetQuestTimerHandle)))

(event Custom|Choose%20Random%20Quest
  (Variables|Default|SetActive%20Quest (.OutItem (Utilities|Array|Random (Variables|Default|GetArray%20of%20quests))))
  (bind _returnvalue (Utilities|Time|SetTimerbyEvent (delegate Custom|QuestTimeout) 2e+01))
  (Variables|Default|SetQuestTimerHandle _returnvalue))

(event Custom|StartQuest
  (params (ActiveHeroes :type Array%20of%20BP%20Base%20Hero%20Object%20References))
  (bind _timetotravel (Default|FindTravelTime (Variables|Default|GetActive%20Quest)))
  (Utilities|Time|SetTimerbyEvent (delegate Custom|OnArrivedAtLocation) _timetotravel))

(event Custom|OnArrivedAtLocation
  (bind _quest_time (Default|FindQuestTime (Variables|Default|GetActive%20Quest)))
  (Utilities|Time|SetTimerbyEvent (delegate Custom|OnCompletedQuest) _quest_time))

(event Custom|OnCompletedQuest
  (bind _newparam (CallFunction|GenerateRandomPoint (.RequiredStats (Utilities|Struct|BreakS_QuestMechanicsInfo (Variables|/Game/Zen/QuestStuff/PDA_QuestData.PDA_QuestData_C|GetMechanics%20Relevant (Variables|Default|GetActive%20Quest))))))
  (bind _isvalid (CallFunction|IsPointValid _newparam))
  (if _isvalid
    (CallFunction|QuestSuccess)
    (else
      (CallFunction|QuestFailed))))

(event Custom|QuestSuccess)

(event Custom|QuestFailed)

(event EventBeginPlay)

(fn ConstructionScript)