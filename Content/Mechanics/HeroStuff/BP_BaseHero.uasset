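; BP_BaseHero is the base hero Blueprint, holding hero info, state and index, with getters for other systems.
; Successes accumulate until they reach a rising threshold, which triggers a level-up.
; Leveling rolls randomly against a running sum of per-stat upgrade chances, re-rolling for each stat, and increments the last stat that passes.
; The highest stat, recomputed at BeginPlay and each level-up, maps to the hero's active skill enum.
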(event EventBeginPlay
  (bind _values (Utilities|Map|Values (.Stats (Utilities|Struct|BreakS_HeroInfo (Variables|Default|GetHero%20Info)))))
  (bind _highest_stat (CallFunction|UpdateActiveSkill _values))
  (Variables|Default|SetHighest%20Stat _highest_stat))

(event EventAddSuccessCounter
  (bind _result (Math|Integer|IncrementInt (Variables|Default|GetSuccess%20Counter))
    (:%20%20
      (if (>= _result (Variables|Default|GetSuccess%20to%20Upgrade%20level))
        (Math|Integer|IncrementInt (Variables|Default|GetSuccess%20to%20Upgrade%20level)
          (:%20%20
            (CallFunction|IncreaseHeroLevel)))))))

(event EventSetHeroState
  (params (New%20State :type E_HeroState%20Enum :default "NewEnumerator0"))
  (Variables|Default|SetHero%20State New%20State))

(fn ConstructionScript)

(fn UpdateActiveSkill
  (params (Hero%20Stats :type Array%20of%20Floats%20%28double-precision%29))
  (switch int (.IndexOfMaxValue (Math|Float|MaxOfFloatArray Hero%20Stats))
    (:0
      (return "NewEnumerator0"))
    (:1
      (return "NewEnumerator1"))
    (:2
      (return "NewEnumerator2"))
    (:3
      (return "NewEnumerator3"))
    (:4
      (return "NewEnumerator4"))))

(fn IncreaseHeroLevel
  (bind _hero_info (Variables|Default|GetHero%20Info))
  (bind _hero_info_2 (Variables|Default|GetHero%20Info))
  (Math|Integer|IncrementInt (.level _hero_info)
    (:%20%20
      (bind _keys (Utilities|Map|Keys (.upgradablestats _hero_info)))
      (for _array_element _keys
        (bind _output_get (LocalVariables|SetPercentage%20Value (+ (LocalVariables|GetPercentage%20Value) (.Value (Utilities|Map|Find (.upgradablestats _hero_info) _array_element)))))
        (if (<= (Math|Random|RandomFloatinRange 0.0 1e+02) _output_get)
          (LocalVariables|SetStat%20to%20Upgrade _array_element)))
      (Math|Float|IncrementFloat (.Value (Utilities|Map|Find (.stats _hero_info_2) (LocalVariables|GetStat%20to%20Upgrade)))
        (:%20%20
          (bind _values (Utilities|Map|Values (.stats _hero_info_2)))
          (bind _highest_stat (CallFunction|UpdateActiveSkill _values))
          (Variables|Default|SetHighest%20Stat _highest_stat))))))

(fn GetHeroBP
  (return self))

(fn GetHeroIndex
  (return (Variables|Default|GetHero%20Index)))

(fn GetHeroStats
  (return (Variables|Default|GetHero%20Info)))

(fn GetHighestStat
  (return (Variables|Default|GetHighest%20Stat)))